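; Base skeleton enemy character that damages the player on overlap and can be hurt or killed.
; Pawn sensing sets a player-seen flag for a State Tree.
; Hits and lethal spikes share one damage path: survivors play a montage and launch away from the player, while the dead drop pawn collision and are destroyed after a delay.
; Unless it sees the player, it flips 180 degrees on turn events, with enemy-overlap turns debounced.
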(event OnSeePawn(PawnSensing)
  (params (Pawn :type Pawn%20Object%20Reference))
  ;[0.15 0.15 0.15 0.5] If sees player set SeeingPlayer? for state tree
  (if (Actor|ActorHasTag Pawn "Player")
    (Variables|Default|SetSeeingPLayer? true)
    (else
      (Variables|Default|SetSeeingPLayer? false))))

(event OnComponentBeginOverlap(Capsule)
  (params (OverlappedComponent :type Primitive%20Component%20Object%20Reference) (OtherActor :type Actor%20Object%20Reference) (OtherComp :type Primitive%20Component%20Object%20Reference) (OtherBodyIndex :type Integer) (bFromSweep :type Boolean) (SweepResult :type Hit%20Result%20Structure%20%28by%20ref%29))
  ;[0.15 0.15 0.15 0.5] If hits player calls hit player interface, if hits another skeleton turns away from skeleton unless chasing player
  (bind _asbp_research_project_character (Utilities|Casting|CastToBP_ResearchProjectCharacter OtherActor)
    (:then
      (Default|HitPlayer _asbp_research_project_character 1 (Transformation|GetWorldLocation (Variables|Collision|GetCapsuleComponent))))
    (:CastFailed
      (if (and (Actor|ActorHasTag OtherActor "Enemy") (!= OtherActor self))
        (if (not (Variables|Default|GetLoopProtection))
          (CallFunction|TurnAround)
          (Variables|Default|SetLoopProtection true)
          (Utilities|FlowControl|Delay 0.5)
          (Variables|Default|SetLoopProtection false))))))

(event Custom|TurnAround
  (bind _capsulecomponent (Variables|Collision|GetCapsuleComponent))
  (bind _charactermovement (Variables|Character|GetCharacterMovement))
  (bind _returnvalue (Transformation|GetWorldRotation _capsulecomponent))
  ;[0.15 0.15 0.15 0.5] Turns player around through event and interface
  (if (not (Variables|Default|GetSeeingPLayer?))
    (Class|NavMovementInterface|StopActiveMovement _charactermovement)
    (Components|Movement|StopMovementImmediately _charactermovement)
    (Transformation|SetWorldRotation _capsulecomponent (Math|Rotator|MakeRotator (.roll _returnvalue) (.pitch _returnvalue) (+ (.yaw _returnvalue) 1.8e+02)) false true)))

(event EventRanIntoSkeleton
  (bind _capsulecomponent (Variables|Collision|GetCapsuleComponent))
  (bind _charactermovement (Variables|Character|GetCharacterMovement))
  (bind _returnvalue (Transformation|GetWorldRotation _capsulecomponent))
  ;[0.15 0.15 0.15 0.5] Turns player around through event and interface
  (if (not (Variables|Default|GetSeeingPLayer?))
    (Class|NavMovementInterface|StopActiveMovement _charactermovement)
    (Components|Movement|StopMovementImmediately _charactermovement)
    (Transformation|SetWorldRotation _capsulecomponent (Math|Rotator|MakeRotator (.roll _returnvalue) (.pitch _returnvalue) (+ (.yaw _returnvalue) 1.8e+02)) false true)))

(event EventTakeSpikeDamageEnemy
  (bind _capsulecomponent (Variables|Collision|GetCapsuleComponent))
  (bind _capsule (Variables|Default|GetCapsule))
  ;[0.15 0.15 0.15 0.5] Take damage events
  ;;[0.15 0.15 0.15 0.5] Take damage from spikes
  (Variables|Default|SetHealth 0)
  (if (> (stale EventHitActor _output_get) 0)
    ;;[0.15 0.15 0.15 0.5] damage anim
    (Animation|Montage|PlayMontage (Variables|Character|GetMesh) "/Game/Characters/Skeletons/MinionAnimations/Rig_Medium_General_Anim_Hit_B_Montage.Rig_Medium_General_Anim_Hit_B_Montage"
      (:then
        (bind _asbp_research_project_character (Utilities|Casting|CastToBP_ResearchProjectCharacter (Game|GetPlayerCharacter 0)))
        ;;[0.15 0.15 0.15 0.5] launch away from players
        (Components|Movement|StopMovementImmediately (Variables|Character|GetCharacterMovement))
        (Character|LaunchCharacter (Math|Vector|MakeVector (* (.x (Math|Vector|GetUnitDirection(Vector) (Transformation|GetWorldLocation (Variables|/Script/Engine.Character|GetCapsuleComponent _asbp_research_project_character)) (Transformation|GetWorldLocation (Variables|Collision|GetCapsuleComponent)))) 3e+02) 0.0 3e+02) false false)))
    (else
      ;;[0.15 0.15 0.15 0.5] plays death anim and disables colision  with pawns
      (Variables|Default|SetIsWalking false)
      (Variables|Default|SetIsRunning false)
      (Variables|Default|SetIsDead true)
      (Animation|Montage|PlayMontage (Variables|Character|GetMesh) "/Game/Characters/Skeletons/MinionAnimations/Rig_Medium_General_Anim_Death_A_Montage.Rig_Medium_General_Anim_Death_A_Montage"
        (:then
          (Components|Movement|StopMovementImmediately (Variables|Character|GetCharacterMovement))
          (Components|Activation|Deactivate (Variables|Default|GetPawnSensing))
          (Collision|SetCollisionResponsetoChannel _capsulecomponent "ECC_Pawn" "ECR_Ignore")
          (Collision|SetCollisionResponsetoChannel _capsulecomponent "ECC_GameTraceChannel3" "ECR_Ignore")
          (Collision|SetCollisionResponsetoChannel _capsule "ECC_Pawn" "ECR_Ignore")
          (Collision|SetCollisionResponsetoChannel _capsule "ECC_GameTraceChannel3" "ECR_Ignore"))
        (:OnCompleted
          (Utilities|FlowControl|Delay 5.0)
          (Actor|DestroyActor))))))

(event EventHitActor
  (params (Damage :type Integer))
  (bind _capsulecomponent (Variables|Collision|GetCapsuleComponent))
  (bind _capsule (Variables|Default|GetCapsule))
  ;[0.15 0.15 0.15 0.5] Take damage events
  ;;[0.15 0.15 0.15 0.5] Take damage from players
  (Variables|Default|SetWasHit true)
  (bind _output_get (Variables|Default|SetHealth (- (Variables|Default|GetHealth) Damage)))
  (if (> _output_get 0)
    ;;[0.15 0.15 0.15 0.5] damage anim
    (Animation|Montage|PlayMontage (Variables|Character|GetMesh) "/Game/Characters/Skeletons/MinionAnimations/Rig_Medium_General_Anim_Hit_B_Montage.Rig_Medium_General_Anim_Hit_B_Montage"
      (:then
        (bind _asbp_research_project_character (Utilities|Casting|CastToBP_ResearchProjectCharacter (Game|GetPlayerCharacter 0)))
        ;;[0.15 0.15 0.15 0.5] launch away from players
        (Components|Movement|StopMovementImmediately (Variables|Character|GetCharacterMovement))
        (Character|LaunchCharacter (Math|Vector|MakeVector (* (.x (Math|Vector|GetUnitDirection(Vector) (Transformation|GetWorldLocation (Variables|/Script/Engine.Character|GetCapsuleComponent _asbp_research_project_character)) (Transformation|GetWorldLocation (Variables|Collision|GetCapsuleComponent)))) 3e+02) 0.0 3e+02) false false)))
    (else
      ;;[0.15 0.15 0.15 0.5] plays death anim and disables colision  with pawns
      (Variables|Default|SetIsWalking false)
      (Variables|Default|SetIsRunning false)
      (Variables|Default|SetIsDead true)
      (Animation|Montage|PlayMontage (Variables|Character|GetMesh) "/Game/Characters/Skeletons/MinionAnimations/Rig_Medium_General_Anim_Death_A_Montage.Rig_Medium_General_Anim_Death_A_Montage"
        (:then
          (Components|Movement|StopMovementImmediately (Variables|Character|GetCharacterMovement))
          (Components|Activation|Deactivate (Variables|Default|GetPawnSensing))
          (Collision|SetCollisionResponsetoChannel _capsulecomponent "ECC_Pawn" "ECR_Ignore")
          (Collision|SetCollisionResponsetoChannel _capsulecomponent "ECC_GameTraceChannel3" "ECR_Ignore")
          (Collision|SetCollisionResponsetoChannel _capsule "ECC_Pawn" "ECR_Ignore")
          (Collision|SetCollisionResponsetoChannel _capsule "ECC_GameTraceChannel3" "ECR_Ignore"))
        (:OnCompleted
          (Utilities|FlowControl|Delay 5.0)
          (Actor|DestroyActor))))))

(fn ConstructionScript)