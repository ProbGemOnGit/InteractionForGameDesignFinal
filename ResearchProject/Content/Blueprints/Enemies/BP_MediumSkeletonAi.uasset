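; Medium skeleton enemy character with an axe that damages the player, takes knockback hits, and dies instantly to spikes.
; Pawn sensing keeps SeesPlayer set via a retriggerable delay; when unset, hits or bumping other enemies can turn it around.
; Two capsules deal hits gated by CanHitPlayer, a third deals ungated contact damage, and a reversible timeline scales axe crystals.
; Death plays a montage, disables sensing and pawn collision, then destroys the actor.
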(event OnSeePawn(PawnSensing)
  (params (Pawn :type Pawn%20Object%20Reference))
  (if (Actor|ActorHasTag Pawn "Player")
    (Utilities|FlowControl|Sequence
      (:then_0
        (Variables|Default|SetSeesPlayer true))
      (:then_1
        (Utilities|FlowControl|RetriggerableDelay 0.6)
        (Variables|Default|SetSeesPlayer false)))))

(event OnComponentBeginOverlap(Capsule)
  (params (OverlappedComponent :type Primitive%20Component%20Object%20Reference) (OtherActor :type Actor%20Object%20Reference) (OtherComp :type Primitive%20Component%20Object%20Reference) (OtherBodyIndex :type Integer) (bFromSweep :type Boolean) (SweepResult :type Hit%20Result%20Structure%20%28by%20ref%29))
  (if (and (Actor|ActorHasTag OtherActor "Player") (Variables|Default|GetCanHitPlayer))
    (Variables|Default|SetCanHitPlayer false)
    (Class|BPIPlayer|HitPlayer(Message) OtherActor 1 (Transformation|GetWorldLocation (Variables|Collision|GetCapsuleComponent)))))

(event OnComponentBeginOverlap(Capsule1)
  (params (OverlappedComponent :type Primitive%20Component%20Object%20Reference) (OtherActor :type Actor%20Object%20Reference) (OtherComp :type Primitive%20Component%20Object%20Reference) (OtherBodyIndex :type Integer) (bFromSweep :type Boolean) (SweepResult :type Hit%20Result%20Structure%20%28by%20ref%29))
  (if (and (Actor|ActorHasTag OtherActor "Player") (Variables|Default|GetCanHitPlayer))
    (Variables|Default|SetCanHitPlayer false)
    (Class|BPIPlayer|HitPlayer(Message) OtherActor 1 (Transformation|GetWorldLocation (Variables|Collision|GetCapsuleComponent)))))

(event OnComponentBeginOverlap(Capsule2)
  (params (OverlappedComponent :type Primitive%20Component%20Object%20Reference) (OtherActor :type Actor%20Object%20Reference) (OtherComp :type Primitive%20Component%20Object%20Reference) (OtherBodyIndex :type Integer) (bFromSweep :type Boolean) (SweepResult :type Hit%20Result%20Structure%20%28by%20ref%29))
  (Utilities|Casting|CastToBP_ResearchProjectCharacter OtherActor
    (:then
      (Class|BPIPlayer|HitPlayer(Message) OtherActor 1 (Transformation|GetWorldLocation (Variables|Collision|GetCapsuleComponent))))
    (:CastFailed
      (if (and (Actor|ActorHasTag OtherActor "Enemy") (!= OtherActor self))
        (CallFunction|TurnAround)
        (Class|BPIISkeleton|RanIntoSkeleton(Message) OtherActor)))))

(event Custom|TurnAround
  (bind _capsulecomponent (Variables|Collision|GetCapsuleComponent))
  (bind _charactermovement (Variables|Character|GetCharacterMovement))
  (bind _returnvalue (Transformation|GetWorldRotation _capsulecomponent))
  (if (and (not (Variables|Default|GetSeesPlayer)) (not (Variables|Default|GetLoop%20Projection)))
    (Variables|Default|SetLoop%20Projection true)
    (Class|NavMovementInterface|StopActiveMovement _charactermovement)
    (Components|Movement|StopMovementImmediately _charactermovement)
    (Transformation|SetWorldRotation _capsulecomponent (Math|Rotator|MakeRotator (.roll _returnvalue) (.pitch _returnvalue) (+ (.yaw _returnvalue) 1.8e+02)) false true)
    (Utilities|FlowControl|Delay 0.5)
    (Variables|Default|SetLoop%20Projection false)))

(event Custom|DespawnAxeCrystals
  (bind _newtrack_0 (Timeline|Timeline ReverseFromEnd)
    (:Update
      (Transformation|SetRelativeScale3D (Variables|Default|GetCrystal1) (Math|Vector|Lerp(Vector) "0, 0, 0" "10.000000,10.000000,25.500000" _newtrack_0)))))

(event Custom|SpawnAxeCrystals
  (bind _newtrack_0 (Timeline|Timeline PlayFromStart)
    (:Update
      (Transformation|SetRelativeScale3D (Variables|Default|GetCrystal1) (Math|Vector|Lerp(Vector) "0, 0, 0" "10.000000,10.000000,25.500000" _newtrack_0)))))

(event EventHitActor
  (params (Damage :type Integer))
  (bind _capsulecomponent (Variables|Collision|GetCapsuleComponent))
  (bind _capsulecomponent_2 (Variables|Collision|GetCapsuleComponent))
  ;[0.15 0.15 0.15 0.5] Take damage from players
  (bind _output_get (Variables|Default|SetHealth (- (Variables|Default|GetHealth) Damage)))
  (Audio|PlaySound2D "/Game/SoundEffects/SkeletonDamageSound.SkeletonDamageSound" 1.0 1.0 0.0 0 0)
  (if (> _output_get 0)
    ;[0.15 0.15 0.15 0.5] damage anim
    (Animation|Montage|PlayMontage (Variables|Character|GetMesh) "/Game/Characters/Skeletons/MinionAnimations/Rig_Medium_General_Anim_Hit_B_Montage.Rig_Medium_General_Anim_Hit_B_Montage"
      (:then
        (bind _asbp_research_project_character (Utilities|Casting|CastToBP_ResearchProjectCharacter (Game|GetPlayerCharacter 0)))
        ;[0.15 0.15 0.15 0.5] launch away from players
        (Components|Movement|StopMovementImmediately (Variables|Character|GetCharacterMovement))
        (Character|LaunchCharacter (Math|Vector|MakeVector (* (.x (Math|Vector|GetUnitDirection(Vector) (Transformation|GetWorldLocation (Variables|/Script/Engine.Character|GetCapsuleComponent _asbp_research_project_character)) (Transformation|GetWorldLocation (Variables|Collision|GetCapsuleComponent)))) 3e+02) 0.0 3e+02) false false)
        (if (not (Variables|Default|GetSeesPlayer))
          (CallFunction|TurnAround))))
    (else
      ;[0.15 0.15 0.15 0.5] plays death anim and disables colision  with pawns
      (Variables|Default|SetIsWalking false)
      (Variables|Default|SetIsRunning false)
      (Variables|Default|SetIsDead true)
      (Animation|Montage|PlayMontage (Variables|Character|GetMesh) "/Game/Characters/Skeletons/MinionAnimations/Rig_Medium_General_Anim_Death_A_Montage.Rig_Medium_General_Anim_Death_A_Montage"
        (:then
          (Components|Movement|StopMovementImmediately (Variables|Character|GetCharacterMovement))
          (Components|Activation|Deactivate (Variables|Default|GetPawnSensing))
          (Collision|SetCollisionResponsetoChannel _capsulecomponent "ECC_Pawn" "ECR_Ignore")
          (Collision|SetCollisionResponsetoChannel _capsulecomponent "ECC_GameTraceChannel3" "ECR_Ignore")
          (Collision|SetCollisionResponsetoChannel _capsulecomponent_2 "ECC_Pawn" "ECR_Ignore")
          (Collision|SetCollisionResponsetoChannel _capsulecomponent_2 "ECC_GameTraceChannel3" "ECR_Ignore"))
        (:OnCompleted
          (Utilities|FlowControl|Delay 5.0)
          (Actor|DestroyActor))))))

(event EventTick
  (params (DeltaSeconds :type Float%20%28single-precision%29))
  (Variables|Default|SetIsFalling (AI|Components|NavMovement|IsFalling (Variables|Character|GetCharacterMovement))))

(event EventRanIntoSkeleton
  (bind _capsulecomponent (Variables|Collision|GetCapsuleComponent))
  (bind _charactermovement (Variables|Character|GetCharacterMovement))
  (bind _returnvalue (Transformation|GetWorldRotation _capsulecomponent))
  (if (and (not (Variables|Default|GetSeesPlayer)) (not (Variables|Default|GetLoop%20Projection)))
    (Variables|Default|SetLoop%20Projection true)
    (Class|NavMovementInterface|StopActiveMovement _charactermovement)
    (Components|Movement|StopMovementImmediately _charactermovement)
    (Transformation|SetWorldRotation _capsulecomponent (Math|Rotator|MakeRotator (.roll _returnvalue) (.pitch _returnvalue) (+ (.yaw _returnvalue) 1.8e+02)) false true)
    (Utilities|FlowControl|Delay 0.5)
    (Variables|Default|SetLoop%20Projection false)))

(event EventTakeSpikeDamageEnemy
  (bind _capsulecomponent (Variables|Collision|GetCapsuleComponent))
  (bind _capsulecomponent_2 (Variables|Collision|GetCapsuleComponent))
  ;[0.15 0.15 0.15 0.5] Take damage from spikes
  (Variables|Default|SetHealth 0)
  (if (> (stale EventHitActor _output_get) 0)
    ;[0.15 0.15 0.15 0.5] damage anim
    (Animation|Montage|PlayMontage (Variables|Character|GetMesh) "/Game/Characters/Skeletons/MinionAnimations/Rig_Medium_General_Anim_Hit_B_Montage.Rig_Medium_General_Anim_Hit_B_Montage"
      (:then
        (bind _asbp_research_project_character (Utilities|Casting|CastToBP_ResearchProjectCharacter (Game|GetPlayerCharacter 0)))
        ;[0.15 0.15 0.15 0.5] launch away from players
        (Components|Movement|StopMovementImmediately (Variables|Character|GetCharacterMovement))
        (Character|LaunchCharacter (Math|Vector|MakeVector (* (.x (Math|Vector|GetUnitDirection(Vector) (Transformation|GetWorldLocation (Variables|/Script/Engine.Character|GetCapsuleComponent _asbp_research_project_character)) (Transformation|GetWorldLocation (Variables|Collision|GetCapsuleComponent)))) 3e+02) 0.0 3e+02) false false)
        (if (not (Variables|Default|GetSeesPlayer))
          (CallFunction|TurnAround))))
    (else
      ;[0.15 0.15 0.15 0.5] plays death anim and disables colision  with pawns
      (Variables|Default|SetIsWalking false)
      (Variables|Default|SetIsRunning false)
      (Variables|Default|SetIsDead true)
      (Animation|Montage|PlayMontage (Variables|Character|GetMesh) "/Game/Characters/Skeletons/MinionAnimations/Rig_Medium_General_Anim_Death_A_Montage.Rig_Medium_General_Anim_Death_A_Montage"
        (:then
          (Components|Movement|StopMovementImmediately (Variables|Character|GetCharacterMovement))
          (Components|Activation|Deactivate (Variables|Default|GetPawnSensing))
          (Collision|SetCollisionResponsetoChannel _capsulecomponent "ECC_Pawn" "ECR_Ignore")
          (Collision|SetCollisionResponsetoChannel _capsulecomponent "ECC_GameTraceChannel3" "ECR_Ignore")
          (Collision|SetCollisionResponsetoChannel _capsulecomponent_2 "ECC_Pawn" "ECR_Ignore")
          (Collision|SetCollisionResponsetoChannel _capsulecomponent_2 "ECC_GameTraceChannel3" "ECR_Ignore"))
        (:OnCompleted
          (Utilities|FlowControl|Delay 5.0)
          (Actor|DestroyActor))))))

(event EventBeginPlay
  (Transformation|AttachComponentToComponent (Variables|Default|GetAxe) (Variables|Character|GetMesh) "hand_rSocket" "SnapToTarget" "SnapToTarget" "KeepRelative" true))

(fn ConstructionScript)