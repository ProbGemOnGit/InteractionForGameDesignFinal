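; Rogue skeleton enemy that patrols with an axe, chases sighted players and deals melee or contact damage.
; Patrol uses forward and downward line traces with AIMoveTo, flipping 180° at obstacles, missing ground or bumped non-player actors.
; PawnSensing starts the chase; the attack montage times a box-overlap swing, while capsule contact damages on a cooldown.
; Hits knock it back and draw it toward the player; death disables sensing and collision responses, then destroys it.
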(event OnSeePawn(PawnSensing)
  (params (Pawn :type Pawn%20Object%20Reference))
  (if (not (Variables|Default|GetIsDead))
    (Variables|Default|SetIsWalking false)
    (Variables|Default|SetIsRunning true)
    (Variables|Default|SetSeesPlayer true)
    (Variables|/Script/Engine.CharacterMovementComponent|SetMaxWalkSpeed (Variables|Character|GetCharacterMovement) 5e+02)
    (AI|AIMoveTo self "0, 0, 0" Pawn 2e+02 false
      (:then
        (Utilities|FlowControl|RetriggerableDelay 2.0)
        (CallFunction|MoveLocation))
      (:OnSuccess
        (CallFunction|AttackPlayer)))))

(event OnComponentBeginOverlap(Capsule)
  (params (OverlappedComponent :type Primitive%20Component%20Object%20Reference) (OtherActor :type Actor%20Object%20Reference) (OtherComp :type Primitive%20Component%20Object%20Reference) (OtherBodyIndex :type Integer) (bFromSweep :type Boolean) (SweepResult :type Hit%20Result%20Structure%20%28by%20ref%29))
  (Utilities|Casting|CastToBP_ResearchProjectCharacter OtherActor
    (:then
      (Variables|Default|SetIsHitingPlayer true)
      (CallFunction|HitPlayer))
    (:CastFailed
      (if (not (Variables|Default|GetLoopProtection))
        (Variables|Default|SetLoopProtection true)
        (Class|BPIISkeleton|RanIntoSkeleton(Message) OtherActor)
        (CallFunction|TurnAround)
        (Utilities|FlowControl|Delay 2.0)
        (Variables|Default|SetLoopProtection false)))))

(event OnComponentEndOverlap(Capsule)
  (params (OverlappedComponent :type Primitive%20Component%20Object%20Reference) (OtherActor :type Actor%20Object%20Reference) (OtherComp :type Primitive%20Component%20Object%20Reference) (OtherBodyIndex :type Integer))
  (Utilities|Casting|CastToBP_ResearchProjectCharacter OtherActor)
  (Variables|Default|SetIsHitingPlayer false))

(event Custom|Move%20Location
  (bind _capsulecomponent (Variables|Collision|GetCapsuleComponent))
  (bind _capsulecomponent_2 (Variables|Collision|GetCapsuleComponent))
  (bind _capsulecomponent_3 (Variables|Collision|GetCapsuleComponent))
  (bind _capsulecomponent_4 (Variables|Collision|GetCapsuleComponent))
  (bind _returnvalue (Transformation|GetWorldRotation _capsulecomponent_3))
  (bind _returnvalue_2 (Transformation|GetWorldLocation _capsulecomponent))
  (bind _returnvalue_3 (Transformation|GetWorldLocation _capsulecomponent_2))
  (bind _returnvalue_4 (Transformation|GetWorldRotation _capsulecomponent_4))
  (Variables|Default|SetSeesPlayer false)
  (if (not (Variables|Default|GetIsDead))
    (Variables|Default|SetIsWalking true)
    (Variables|Default|SetIsRunning false)
    (if (not (AI|Components|NavMovement|IsFalling (Variables|Character|GetCharacterMovement)))
      (Variables|/Script/Engine.CharacterMovementComponent|SetMaxWalkSpeed (Variables|Character|GetCharacterMovement) 275.0)
      (bind (_outhit _returnvalue_5) (Collision|LineTraceByChannel (Math|Vector|MakeVector (.x _returnvalue_3) (.y _returnvalue_3) (+ (.z _returnvalue_3) 5e+01)) (+ (Math|Vector|MakeVector (.x _returnvalue_3) (.y _returnvalue_3) (.z _returnvalue_3)) (* (Math|Vector|GetForwardVector _capsulecomponent_2) 2.5e+02)) "TraceTypeQuery1" false 0 "None"))
      (if _returnvalue_5
        (AI|AIMoveTo self (.Location (Collision|BreakHitResult _outhit)) 0 5.0 false
          (:OnSuccess
            (Transformation|SetWorldRotation _capsulecomponent_4 (Math|Rotator|MakeRotator (.roll _returnvalue_4) (.pitch _returnvalue_4) (+ (.yaw _returnvalue_4) 1.8e+02)) false false)
            (CallFunction|MoveLocation)))
        (else
          (bind (_outhit_2 _returnvalue_6) (Collision|LineTraceByChannel (Math|Vector|MakeVector (.x _returnvalue_2) (.y _returnvalue_2) (+ (.z _returnvalue_2) 5e+01)) (+ (Math|Vector|MakeVector (.x _returnvalue_2) (.y _returnvalue_2) (- (.z _returnvalue_2) 1.2e+02)) (* (Math|Vector|GetForwardVector _capsulecomponent) 1e+02)) "TraceTypeQuery1" false 0 "None"))
          (if _returnvalue_6
            (AI|AIMoveTo self (.Location (Collision|BreakHitResult _outhit_2)) 0 0.1 false
              (:OnSuccess
                _)
              (:OnFail
                _))
            (CallFunction|MoveLocation)
            (else
              (Transformation|SetWorldRotation _capsulecomponent_3 (Math|Rotator|MakeRotator (.roll _returnvalue) (.pitch _returnvalue) (+ (.yaw _returnvalue) 1.8e+02)) false false)
              (CallFunction|MoveLocation))))))))

(event Custom|HitPlayer
  (if (not (Variables|Default|GetIsDead))
    (if (not (Variables|Default|GetHitCooldown))
      (Variables|Default|SetHitCooldown true)
      (bind _asbp_research_project_character (Utilities|Casting|CastToBP_ResearchProjectCharacter (Game|GetPlayerCharacter 0)))
      (Default|HitPlayer _asbp_research_project_character 1 (Transformation|GetActorLocation))
      (Components|Activation|Deactivate (Variables|Default|GetPawnSensing))
      (Components|Movement|StopMovementImmediately (Variables|Character|GetCharacterMovement))
      (Variables|Default|SetIsRunning false)
      (Variables|Default|SetIsWalking false)
      (Utilities|Time|SetTimerbyEvent (delegate Custom|TryHitPlayer) 2.2))))

(event Custom|TryHitPlayer
  (Components|Activation|Activate (Variables|Default|GetPawnSensing) false)
  (Variables|Default|SetHitCooldown false)
  (if (and (Variables|Default|GetIsHitingPlayer) (not (Variables|Default|GetIsDead)))
    (CallFunction|HitPlayer)))

(event Custom|AttackPlayer
  (if (not (Variables|Default|GetAttackCoolDown))
    (Variables|Default|SetAttackCoolDown true)
    (Variables|Default|SetIsRunning false)
    (Variables|Default|SetIsWalking false)
    (Variables|Default|SetIsHitting true)
    (Components|Movement|StopMovementImmediately (Variables|Character|GetCharacterMovement))
    (Animation|Montage|PlayMontage (Variables|Character|GetMesh) "/Game/Characters/Skeletons/RogueAnimation/Rig_Medium_General_Anim_Throw_Montage.Rig_Medium_General_Anim_Throw_Montage"
      (:then
        (Utilities|Time|SetTimerbyEvent (delegate Custom|Swing) 0.5))
      (:OnCompleted
        (Utilities|FlowControl|Delay 0.5)
        (Variables|Default|SetIsHitting false)
        (Variables|Default|SetAttackCoolDown false)
        (if (not (Variables|Default|GetSeesPlayer))
          (CallFunction|MoveLocation))))))

(event Custom|Swing
  (for _array_element (Collision|GetOverlappingActors (Variables|Default|GetBox) 0 :!class /Script/Engine.PrimitiveComponent)
    (Class|BPIPlayer|HitPlayer(Message) _array_element 1 (Transformation|GetActorLocation))))

(event Custom|TurnAround
  (bind _capsulecomponent (Variables|Collision|GetCapsuleComponent))
  (bind _returnvalue (Transformation|GetWorldRotation _capsulecomponent))
  (Transformation|SetWorldRotation _capsulecomponent (Math|Rotator|MakeRotator (.roll _returnvalue) (.pitch _returnvalue) (+ (.yaw _returnvalue) 1.8e+02)) false false))

(event EventBeginPlay
  (Transformation|AttachComponentToComponent (Variables|Default|GetAxe) (Variables|Character|GetMesh) "hand_rSocket" "SnapToTarget" "SnapToTarget" "KeepWorld" true)
  (if (Variables|Default|GetStartsMoving)
    (CallFunction|MoveLocation)))

(event EventTakeSpikeDamageEnemy
  (bind _capsulecomponent (Variables|Collision|GetCapsuleComponent))
  (bind _capsulecomponent_2 (Variables|Collision|GetCapsuleComponent))
  (bind _capsule (Variables|Default|GetCapsule))
  (bind _returnvalue (Transformation|GetWorldRotation _capsulecomponent_2))
  (Variables|Default|SetHealth 0)
  (if (> (stale EventHitActor _output_get) 0)
    (Animation|Montage|PlayMontage (Variables|Character|GetMesh) "/Game/Characters/Skeletons/MinionAnimations/Rig_Medium_General_Anim_Hit_B_Montage.Rig_Medium_General_Anim_Hit_B_Montage"
      (:then
        (bind _asbp_research_project_character (Utilities|Casting|CastToBP_ResearchProjectCharacter (Game|GetPlayerCharacter 0)))
        (Components|Movement|StopMovementImmediately (Variables|Character|GetCharacterMovement))
        (Character|LaunchCharacter (Math|Vector|MakeVector (* (.x (Math|Vector|GetUnitDirection(Vector) (Transformation|GetWorldLocation (Variables|/Script/Engine.Character|GetCapsuleComponent _asbp_research_project_character)) (Transformation|GetWorldLocation (Variables|Character|GetMesh)))) 3e+02) 0.0 3e+02) false false)
        (if (not (Variables|Default|GetSeesPlayer))
          (bind _asbp_research_project_character_2 (Utilities|Casting|CastToBP_ResearchProjectCharacter (Game|GetPlayerCharacter 0)))
          (AI|AIMoveTo self "0, 0, 0" _asbp_research_project_character_2 2e+02 false
            (:then
              (Utilities|FlowControl|Delay 2.0)
              (if (not (Variables|Default|GetIsHitting))
                (CallFunction|MoveLocation)))
            (:OnSuccess
              (if (> (.x (Math|Vector|Normalize (Math|Vector|MakeVector (.x (Math|Vector|GetUnitDirection(Vector) (Transformation|GetWorldLocation (Variables|/Script/Engine.Character|GetCapsuleComponent _asbp_research_project_character_2)) (Transformation|GetWorldLocation (Variables|Character|GetMesh)))) (.y (Math|Vector|GetUnitDirection(Vector) (Transformation|GetWorldLocation (Variables|/Script/Engine.Character|GetCapsuleComponent _asbp_research_project_character_2)) (Transformation|GetWorldLocation (Variables|Character|GetMesh)))) 0.0))) 0.0)
                (Transformation|SetWorldRotation _capsulecomponent_2 (Math|Rotator|MakeRotator (.roll _returnvalue) (.pitch _returnvalue) (+ (.yaw _returnvalue) 1.8e+02)) false false)
                (CallFunction|AttackPlayer)))))))
    (else
      (Variables|Default|SetIsWalking false)
      (Variables|Default|SetIsRunning false)
      (Variables|Default|SetIsDead true)
      (Animation|Montage|PlayMontage (Variables|Character|GetMesh) "/Game/Characters/Skeletons/MinionAnimations/Rig_Medium_General_Anim_Death_A_Montage.Rig_Medium_General_Anim_Death_A_Montage"
        (:then
          (Components|Movement|StopMovementImmediately (Variables|Character|GetCharacterMovement))
          (Components|Activation|Deactivate (Variables|Default|GetPawnSensing))
          (Collision|SetCollisionResponsetoChannel _capsulecomponent "ECC_Pawn" "ECR_Ignore")
          (Collision|SetCollisionResponsetoChannel _capsulecomponent "ECC_GameTraceChannel3" "ECR_Ignore")
          (Collision|SetCollisionResponsetoChannel _capsule "ECC_Pawn" "ECR_Ignore")
          (Collision|SetCollisionResponsetoChannel _capsule "ECC_GameTraceChannel3" "ECR_Ignore"))
        (:OnCompleted
          (Utilities|FlowControl|Delay 5.0)
          (Actor|DestroyActor))))))

(event EventRanIntoSkeleton
  (bind _capsulecomponent (Variables|Collision|GetCapsuleComponent))
  (bind _returnvalue (Transformation|GetWorldRotation _capsulecomponent))
  (Transformation|SetWorldRotation _capsulecomponent (Math|Rotator|MakeRotator (.roll _returnvalue) (.pitch _returnvalue) (+ (.yaw _returnvalue) 1.8e+02)) false false))

(event EventHitActor
  (params (Damage :type Integer))
  (bind _capsulecomponent (Variables|Collision|GetCapsuleComponent))
  (bind _capsulecomponent_2 (Variables|Collision|GetCapsuleComponent))
  (bind _capsule (Variables|Default|GetCapsule))
  (bind _returnvalue (Transformation|GetWorldRotation _capsulecomponent_2))
  (bind _output_get (Variables|Default|SetHealth (- (Variables|Default|GetHealth) Damage)))
  (if (> _output_get 0)
    (Animation|Montage|PlayMontage (Variables|Character|GetMesh) "/Game/Characters/Skeletons/MinionAnimations/Rig_Medium_General_Anim_Hit_B_Montage.Rig_Medium_General_Anim_Hit_B_Montage"
      (:then
        (bind _asbp_research_project_character (Utilities|Casting|CastToBP_ResearchProjectCharacter (Game|GetPlayerCharacter 0)))
        (Components|Movement|StopMovementImmediately (Variables|Character|GetCharacterMovement))
        (Character|LaunchCharacter (Math|Vector|MakeVector (* (.x (Math|Vector|GetUnitDirection(Vector) (Transformation|GetWorldLocation (Variables|/Script/Engine.Character|GetCapsuleComponent _asbp_research_project_character)) (Transformation|GetWorldLocation (Variables|Character|GetMesh)))) 3e+02) 0.0 3e+02) false false)
        (if (not (Variables|Default|GetSeesPlayer))
          (bind _asbp_research_project_character_2 (Utilities|Casting|CastToBP_ResearchProjectCharacter (Game|GetPlayerCharacter 0)))
          (AI|AIMoveTo self "0, 0, 0" _asbp_research_project_character_2 2e+02 false
            (:then
              (Utilities|FlowControl|Delay 2.0)
              (if (not (Variables|Default|GetIsHitting))
                (CallFunction|MoveLocation)))
            (:OnSuccess
              (if (> (.x (Math|Vector|Normalize (Math|Vector|MakeVector (.x (Math|Vector|GetUnitDirection(Vector) (Transformation|GetWorldLocation (Variables|/Script/Engine.Character|GetCapsuleComponent _asbp_research_project_character_2)) (Transformation|GetWorldLocation (Variables|Character|GetMesh)))) (.y (Math|Vector|GetUnitDirection(Vector) (Transformation|GetWorldLocation (Variables|/Script/Engine.Character|GetCapsuleComponent _asbp_research_project_character_2)) (Transformation|GetWorldLocation (Variables|Character|GetMesh)))) 0.0))) 0.0)
                (Transformation|SetWorldRotation _capsulecomponent_2 (Math|Rotator|MakeRotator (.roll _returnvalue) (.pitch _returnvalue) (+ (.yaw _returnvalue) 1.8e+02)) false false)
                (CallFunction|AttackPlayer)))))))
    (else
      (Variables|Default|SetIsWalking false)
      (Variables|Default|SetIsRunning false)
      (Variables|Default|SetIsDead true)
      (Animation|Montage|PlayMontage (Variables|Character|GetMesh) "/Game/Characters/Skeletons/MinionAnimations/Rig_Medium_General_Anim_Death_A_Montage.Rig_Medium_General_Anim_Death_A_Montage"
        (:then
          (Components|Movement|StopMovementImmediately (Variables|Character|GetCharacterMovement))
          (Components|Activation|Deactivate (Variables|Default|GetPawnSensing))
          (Collision|SetCollisionResponsetoChannel _capsulecomponent "ECC_Pawn" "ECR_Ignore")
          (Collision|SetCollisionResponsetoChannel _capsulecomponent "ECC_GameTraceChannel3" "ECR_Ignore")
          (Collision|SetCollisionResponsetoChannel _capsule "ECC_Pawn" "ECR_Ignore")
          (Collision|SetCollisionResponsetoChannel _capsule "ECC_GameTraceChannel3" "ECR_Ignore"))
        (:OnCompleted
          (Utilities|FlowControl|Delay 5.0)
          (Actor|DestroyActor))))))

(fn ConstructionScript)