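; Skeleton enemy Blueprint that paces back and forth, starting on BeginPlay.
; The custom Move event slides the root with MoveComponentTo, then calls itself with a new target 100 units along the mesh's forward X, keeping Y and Z.
; After each step, a short raised Visibility line trace checks ahead, and a hit prints a debug message and yaws the mesh 180 degrees.
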(event Custom|Move
  (params (NewLocation :type Vector))
  (bind _staticmesh (Variables|Default|GetStaticMesh))
  (bind _staticmesh_2 (Variables|Default|GetStaticMesh))
  (bind _staticmesh_3 (Variables|Default|GetStaticMesh))
  (bind _returnvalue (Transformation|GetWorldLocation _staticmesh_2))
  (bind _returnvalue_2 (Transformation|GetWorldLocation _staticmesh_3))
  (bind _returnvalue_3 (Transformation|GetWorldRotation _staticmesh))
  (bind _returnvalue_4 (Transformation|GetWorldLocation _staticmesh_2))
  (Components|MoveComponentTo (Variables|Default|GetDefaultSceneRoot) NewLocation (Transformation|GetWorldRotation (Variables|Default|GetStaticMesh)) false false 0.2 false)
  (bind (_outhit _returnvalue_5) (Collision|LineTraceByChannel (Math|Vector|MakeVector (.x _returnvalue_4) (.y _returnvalue_4) (+ (.z _returnvalue_4) 5e+01)) (+ (Math|Vector|MakeVector (.x _returnvalue) (.y _returnvalue) (+ (.z _returnvalue) 5e+01)) (* (Math|Vector|GetForwardVector _staticmesh_2) 1.5e+02)) "TraceTypeQuery1" false 0 "ForOneFrame"))
  (if _returnvalue_5
    (Development|PrintString "Hello")
    (Transformation|SetWorldRotation _staticmesh (Math|Rotator|MakeRotator (.roll _returnvalue_3) (.pitch _returnvalue_3) (+ (.yaw _returnvalue_3) 1.8e+02)) false false))
  (CallFunction|Move (Math|Vector|MakeVector (+ (.x _returnvalue_2) (* 1e+02 (.x (Math|Vector|GetForwardVector _staticmesh_3)))) (.y _returnvalue_2) (.z _returnvalue_2))))

(event EventBeginPlay
  (bind _staticmesh (Variables|Default|GetStaticMesh))
  (bind _returnvalue (Transformation|GetWorldLocation _staticmesh))
  (CallFunction|Move (Math|Vector|MakeVector (+ (.x _returnvalue) (* 1e+02 (.x (Math|Vector|GetForwardVector _staticmesh)))) (.y _returnvalue) (.z _returnvalue))))

(fn ConstructionScript)