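; BP_TestDummy is an enemy test dummy that reacts to hits and notifies actors whose body overlaps it.
; HitActor sets Health to Damage minus Health, a reversed subtraction, then prints it and plays a hit montage on the skeletal mesh.
; Capsule overlaps check the other component for a "Body" tag, print it and call HitPlayerMessage on that actor with a zero value.
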(event OnComponentBeginOverlap(Capsule)
  (params (OverlappedComponent :type Primitive%20Component%20Object%20Reference) (OtherActor :type Actor%20Object%20Reference) (OtherComp :type Primitive%20Component%20Object%20Reference) (OtherBodyIndex :type Integer) (bFromSweep :type Boolean) (SweepResult :type Hit%20Result%20Structure%20%28by%20ref%29))
  (for _array_element (Variables|/Script/Engine.ActorComponent|GetComponentTags OtherComp)
    (if (== _array_element "Body")
      (Development|PrintString (Utilities|String|ToString(Name) _array_element))
      (Class|BPIPlayer|HitPlayer(Message) OtherActor))))

(event EventHitActor
  (params (Damage :type Integer))
  (bind _output_get (Variables|Default|SetHealth (- Damage (Variables|Default|GetHealth))))
  (Development|PrintString (Utilities|String|ToString(Integer) _output_get))
  (Animation|Montage|PlayMontage (Variables|Default|GetSkeletalMesh) "/Game/Characters/Skeletons/Animations/Rig_Medium_General_Anim_Hit_B_Montage.Rig_Medium_General_Anim_Hit_B_Montage"))

(fn ConstructionScript)