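; BP_AbilityPickUp is a level pickup that unlocks one movement ability for the player character: slide, air dash, wall jump or slide jump.
; BeginPlay sets its static mesh from the configured AbilityMesh.
; On sphere overlap by BP_ResearchProjectCharacter, it switches on AbilityToActivate to set the matching flag on the PlatformerMovementComponent.
; It then adds that ability's pickup widget to the viewport and destroys itself.
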(event OnComponentBeginOverlap(Sphere)
  (params (OverlappedComponent :type Primitive%20Component%20Object%20Reference) (OtherActor :type Actor%20Object%20Reference) (OtherComp :type Primitive%20Component%20Object%20Reference) (OtherBodyIndex :type Integer) (bFromSweep :type Boolean) (SweepResult :type Hit%20Result%20Structure%20%28by%20ref%29))
  (bind _asbp_research_project_character (Utilities|Casting|CastToBP_ResearchProjectCharacter OtherActor))
  (bind _asplatformer_movement_component (Utilities|Casting|CastToPlatformerMovementComponent (Variables|/Script/Engine.Character|GetCharacterMovement _asbp_research_project_character)))
  (switch Utilities|FlowControl|Switch|SwitchonE_Abilities (Variables|Default|GetAbilityToActivate)
    (:NewEnumerator0
      (Variables|/Script/ResearchProject.PlatformerMovementComponent|SetHasSlide _asplatformer_movement_component true)
      (Variables|Default|SetClass "/Game/UI/PickUps/WB_SlidePickUp.WB_SlidePickUp_C"))
    (:NewEnumerator1
      (Variables|/Script/ResearchProject.PlatformerMovementComponent|SetHasAirDash _asplatformer_movement_component true)
      (Variables|Default|SetClass "/Game/UI/PickUps/WB_AirDashPickUp.WB_AirDashPickUp_C"))
    (:NewEnumerator2
      (Variables|/Script/ResearchProject.PlatformerMovementComponent|SetHasWallJump _asplatformer_movement_component true)
      (Variables|Default|SetClass "/Game/UI/PickUps/WB_WallJumpPickUp.WB_WallJumpPickUp_C"))
    (:NewEnumerator3
      (Variables|/Script/ResearchProject.PlatformerMovementComponent|SetHasSlideJump _asplatformer_movement_component true)
      (Variables|Default|SetClass "/Game/UI/PickUps/WB_SlideJumpPickUp.WB_SlideJumpPickUp_C")))
  (bind _returnvalue (UserInterface|CreateWidget (Variables|Default|GetClass)))
  (UserInterface|Viewport|AddtoViewport _returnvalue 0)
  (Actor|DestroyActor))

(event EventBeginPlay
  (Components|StaticMesh|SetStaticMesh (Variables|Default|GetStaticMesh) (Variables|Default|GetAbilityMesh)))

(fn ConstructionScript)