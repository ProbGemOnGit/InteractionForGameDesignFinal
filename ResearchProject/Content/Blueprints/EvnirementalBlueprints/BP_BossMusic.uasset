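; Boss music trigger that plays an intro track followed by a looping track when an actor tagged Player enters its box.
; The intro fades in, then its finished event spawns the loop sound, which respawns on finishing while MusicIsPlaying is set.
; StopMusic clears that flag and fades out the current sound.
; Neither box re-entry nor the intro-to-loop handoff checks the flag.
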(event OnComponentBeginOverlap(Box)
  (params (OverlappedComponent :type Primitive%20Component%20Object%20Reference) (OtherActor :type Actor%20Object%20Reference) (OtherComp :type Primitive%20Component%20Object%20Reference) (OtherBodyIndex :type Integer) (bFromSweep :type Boolean) (SweepResult :type Hit%20Result%20Structure%20%28by%20ref%29))
  (if (Actor|ActorHasTag OtherActor "Player")
    (Variables|Default|SetMusicIsPlaying true)
    (bind _returnvalue (Audio|SpawnSound2D (Variables|Default|GetSound_Start) 1.0 1.0 0.0 0))
    (Variables|Default|SetMusic _returnvalue)
    (Audio|Components|Audio|FadeIn _returnvalue 1.0 1.0 0.0 "Linear" :!class /Script/Engine.AudioComponent)
    (EventDispatchers|AssignOnAudioFinished _returnvalue (delegate Custom|OnAudioFinished_Event))))

(event Custom|OnAudioFinished_Event
  (bind _returnvalue (Audio|SpawnSound2D (Variables|Default|GetSound_Loop) 1.0 1.0 0.0 0))
  (Variables|Default|SetMusic _returnvalue)
  (EventDispatchers|AssignOnAudioFinished _returnvalue (delegate Custom|OnAudioFinished_Event_0)))

(event Custom|OnAudioFinished_Event_0
  (CallFunction|RestartLoop))

(event Custom|RestartLoop
  (if (Variables|Default|GetMusicIsPlaying)
    (bind _returnvalue (Audio|SpawnSound2D (Variables|Default|GetSound_Loop) 1.0 1.0 0.0 0))
    (Variables|Default|SetMusic _returnvalue)
    (EventDispatchers|AssignOnAudioFinished _returnvalue (delegate Custom|OnAudioFinished_Event_0))))

(event Custom|StopMusic
  (if (Variables|Default|GetMusicIsPlaying)
    (Variables|Default|SetMusicIsPlaying false)
    (Audio|Components|Audio|FadeOut (Variables|Default|GetMusic) 2.0 0.0 "Linear" :!class /Script/Engine.AudioComponent)))

(fn ConstructionScript)