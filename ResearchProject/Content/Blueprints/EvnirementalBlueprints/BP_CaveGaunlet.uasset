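; Cave gauntlet encounter that locks the player in with skeleton and base enemy waves, once per save.
; When the player first enters the box, two BP_Platform walls spawn and a five-second recurring check begins.
; Whenever no Enemy-tagged actor overlaps the box, the next wave spawns, counting WaveNum down.
; At zero, it removes the walls, saves SecondGauntletCompleted and destroys itself; BeginPlay also destroys it if already completed.
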(event OnComponentBeginOverlap(Box)
  (params (OverlappedComponent :type Primitive%20Component%20Object%20Reference) (OtherActor :type Actor%20Object%20Reference) (OtherComp :type Primitive%20Component%20Object%20Reference) (OtherBodyIndex :type Integer) (bFromSweep :type Boolean) (SweepResult :type Hit%20Result%20Structure%20%28by%20ref%29))
  (if (Actor|ActorHasTag OtherActor "Player")
    (Utilities|FlowControl|DoOnce false
      (:Completed
        (bind _returnvalue (Game|SpawnActorfromClass "/Game/Blueprints/EvnirementalBlueprints/BP_Platform.BP_Platform_C" (Math|Transform|MakeTransform (Variables|Default|GetWallLocation2) "0, 0, 0" (Variables|Default|GetWallSize2)) "Undefined" "MultiplyWithRoot" 0 0))
        (Variables|Default|SetWall2 _returnvalue)
        (bind _returnvalue_2 (Game|SpawnActorfromClass "/Game/Blueprints/EvnirementalBlueprints/BP_Platform.BP_Platform_C" (Math|Transform|MakeTransform (Variables|Default|GetWallLocation) "0, 0, 0" (Variables|Default|GetWallSize)) "Undefined" "MultiplyWithRoot" 0 0))
        (Variables|Default|SetWall _returnvalue_2)
        (CallFunction|CheckforEnemy)))))

(event Custom|StartWave
  (bind _wavenum (Variables|Default|GetWaveNum))
  (bind _wall (Variables|Default|GetWall))
  (bind _wall2 (Variables|Default|GetWall2))
  (if (> _wavenum 0)
    (switch int _wavenum
      (:1
        (Math|Integer|DecrementInt (Variables|Default|GetWaveNum)
          (:%20%20
            (Game|SpawnActorfromClass "/Game/Blueprints/Enemies/BP_MediumSkeletonAi.BP_MediumSkeletonAi_C" (Math|Transform|MakeTransform (Transformation|GetWorldLocation (Variables|Default|GetSpawn1)) "0, 0, 0" "1.000000,1.000000,1.000000") "Undefined" "MultiplyWithRoot" 0 0)
            (Game|SpawnActorfromClass "/Game/Blueprints/Enemies/BP_MediumSkeletonAi.BP_MediumSkeletonAi_C" (Math|Transform|MakeTransform (Transformation|GetWorldLocation (Variables|Default|GetSpawn2)) "0, 0, 0" "1.000000,1.000000,1.000000") "Undefined" "MultiplyWithRoot" 0 0)
            (Game|SpawnActorfromClass "/Game/Blueprints/Enemies/BP_BaseEnemyAi.BP_BaseEnemyAi_C" (Math|Transform|MakeTransform (Transformation|GetWorldLocation (Variables|Default|GetSpawn3)) "0, 0, 0" "1.000000,1.000000,1.000000") "Undefined" "MultiplyWithRoot" 0 0))))
      (:2
        (Math|Integer|DecrementInt (Variables|Default|GetWaveNum)
          (:%20%20
            (Game|SpawnActorfromClass "/Game/Blueprints/Enemies/BP_BaseEnemyAi.BP_BaseEnemyAi_C" (Math|Transform|MakeTransform (Transformation|GetWorldLocation (Variables|Default|GetSpawn1)) "0, 0, 0" "1.000000,1.000000,1.000000") "Undefined" "MultiplyWithRoot" 0 0)
            (Game|SpawnActorfromClass "/Game/Blueprints/Enemies/BP_BaseEnemyAi.BP_BaseEnemyAi_C" (Math|Transform|MakeTransform (Transformation|GetWorldLocation (Variables|Default|GetSpawn2)) "0, 0, 0" "1.000000,1.000000,1.000000") "Undefined" "MultiplyWithRoot" 0 0)
            (Game|SpawnActorfromClass "/Game/Blueprints/Enemies/BP_BaseEnemyAi.BP_BaseEnemyAi_C" (Math|Transform|MakeTransform (Transformation|GetWorldLocation (Variables|Default|GetSpawn3)) "0, 0, 0" "1.000000,1.000000,1.000000") "Undefined" "MultiplyWithRoot" 0 0))))
      (:3
        (Math|Integer|DecrementInt (Variables|Default|GetWaveNum)
          (:%20%20
            (Game|SpawnActorfromClass "/Game/Blueprints/Enemies/BP_MediumSkeletonAi.BP_MediumSkeletonAi_C" (Math|Transform|MakeTransform (Transformation|GetWorldLocation (Variables|Default|GetSpawn1)) "0, 0, 0" "1.000000,1.000000,1.000000") "Undefined" "MultiplyWithRoot" 0 0)
            (Game|SpawnActorfromClass "/Game/Blueprints/Enemies/BP_MediumSkeletonAi.BP_MediumSkeletonAi_C" (Math|Transform|MakeTransform (Transformation|GetWorldLocation (Variables|Default|GetSpawn3)) "0, 0, 0" "1.000000,1.000000,1.000000") "Undefined" "MultiplyWithRoot" 0 0)))))
    (else
      (Utilities|IsValid _wall
        (:Is%20Valid
          (Actor|DestroyActor _wall)
          (Utilities|IsValid _wall2
            (:Is%20Valid
              (Actor|DestroyActor _wall2)
              (bind _returnvalue (SaveGame|LoadGamefromSlot "Save"))
              (bind _assg_save_data (Utilities|Casting|CastToSG_SaveData _returnvalue))
              (Variables|/Game/Blueprints/SaveGame/SG_SaveData.SG_SaveData_C|SetSecondGauntletCompleted _assg_save_data true)
              (SaveGame|SaveGametoSlot _assg_save_data "Save")
              (Actor|DestroyActor))))))))

(event Custom|CheckForEnemy
  (Variables|Default|SetFoundEnemy false)
  (for _array_element (Collision|GetOverlappingActors (Variables|Default|GetBox) 0 :!class /Script/Engine.PrimitiveComponent)
    (if (Actor|ActorHasTag _array_element "Enemy")
      (Variables|Default|SetFoundEnemy true)))
  (if (Variables|Default|GetFoundEnemy)
    _
    (else
      (CallFunction|StartWave)))
  (Utilities|Time|SetTimerbyEvent (delegate Custom|LoopCheck) 5.0))

(event Custom|LoopCheck
  (CallFunction|CheckforEnemy))

(event EventBeginPlay
  (bind _returnvalue (SaveGame|LoadGamefromSlot "Save"))
  (bind _assg_save_data (Utilities|Casting|CastToSG_SaveData _returnvalue))
  (if (Variables|/Game/Blueprints/SaveGame/SG_SaveData.SG_SaveData_C|GetSecondGauntletCompleted _assg_save_data)
    (Actor|DestroyActor)))

(fn ConstructionScript)