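; BP_DestoryDoors is a destructible environment door that owns a set of platforms, all removed when it is hit.
; On BeginPlay it spawns a BP_Platform at each transform in Platforms and stores the references.
; The HitActor event, guarded by CanHitObject to fire only once, plays a metal clang, then destroys the spawned platforms and the door itself.
; GetDoorName exposes the door's DoorName.
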(event EventBeginPlay
  (for _array_element (Variables|Default|GetPlatforms)
    (bind _returnvalue (Game|SpawnActorfromClass "/Game/Blueprints/EvnirementalBlueprints/BP_Platform.BP_Platform_C" _array_element "Undefined" "MultiplyWithRoot" 0 0))
    (Utilities|Array|Add (Variables|Default|GetSpawnPlatforms) _returnvalue)))

(event EventHitActor
  (params (Damage :type Integer))
  (if (Variables|Default|GetCanHitObject)
    (Variables|Default|SetCanHitObject false)
    (Audio|PlaySound2D "/Game/SoundEffects/metal_clang.metal_clang" 1.0 1.0 0.0 0 0)
    (for _array_element (Variables|Default|GetSpawnPlatforms)
      (Actor|DestroyActor _array_element))
    (Actor|DestroyActor)))

(fn ConstructionScript)

(fn GetDoorName
  (return (Variables|Default|GetDoorName)))