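; BP_Gauntlet is an enemy wave arena trigger, though its wave logic is currently disconnected.
; When a Player enters the box, CheckForEnemy scans it for Enemy-tagged actors and re-checks every five seconds by timer.
; An empty box calls StartWave, an empty event.
; Unwired nodes hold the three-wave countdown spawning skeletons and basic enemies, then removing doors, stopping boss music and destroying the actor.
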(event OnComponentBeginOverlap(Box)
  (params (OverlappedComponent :type Primitive%20Component%20Object%20Reference) (OtherActor :type Actor%20Object%20Reference) (OtherComp :type Primitive%20Component%20Object%20Reference) (OtherBodyIndex :type Integer) (bFromSweep :type Boolean) (SweepResult :type Hit%20Result%20Structure%20%28by%20ref%29))
  (if (Actor|ActorHasTag OtherActor "Player")
    (CallFunction|CheckforEnemy)))

(event Custom|StartWave)

(event Custom|CheckForEnemy
  (Variables|Default|SetFoundEnemy false)
  (for _array_element (Collision|GetOverlappingActors (Variables|Default|GetBox) 0 :!class /Script/Engine.PrimitiveComponent)
    (if (Actor|ActorHasTag _array_element "Enemy")
      (Variables|Default|SetFoundEnemy true)))
  (if (Variables|Default|GetFoundEnemy)
    _
    (else
      (CallFunction|StartWave)))
  (Utilities|Time|SetTimerbyEvent (delegate Custom|LoopCheck) 5.0))

(event Custom|LoopCheck
  (CallFunction|CheckforEnemy))

(fn ConstructionScript)