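; BP_HealthUpgrade is a one-time pickup that raises the player's health heal amount.
; On BeginPlay it destroys itself if the "Save" slot already holds an upgraded HealthHealAMT.
; When BP_ResearchProjectCharacter overlaps its sphere, it writes the higher value to both the save and the character, shows an upgrade popup widget, then destroys itself.
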(event OnComponentBeginOverlap(Sphere)
  (params (OverlappedComponent :type Primitive%20Component%20Object%20Reference) (OtherActor :type Actor%20Object%20Reference) (OtherComp :type Primitive%20Component%20Object%20Reference) (OtherBodyIndex :type Integer) (bFromSweep :type Boolean) (SweepResult :type Hit%20Result%20Structure%20%28by%20ref%29))
  (bind _asbp_research_project_character (Utilities|Casting|CastToBP_ResearchProjectCharacter OtherActor))
  (bind _returnvalue (SaveGame|LoadGamefromSlot "Save"))
  (bind _assg_save_data (Utilities|Casting|CastToSG_SaveData _returnvalue))
  (Variables|/Game/Blueprints/SaveGame/SG_SaveData.SG_SaveData_C|SetHealthHealAMT _assg_save_data 4)
  (SaveGame|SaveGametoSlot _returnvalue "Save")
  (Variables|/Game/Blueprints/Characters/BP_ResearchProjectCharacter.BP_ResearchProjectCharacter_C|SetHealthHealAMT _asbp_research_project_character 4)
  (bind _returnvalue_2 (UserInterface|CreateWidget "/Game/UI/PickUps/WB_HealthUpgradePopup1.WB_HealthUpgradePopup1_C"))
  (UserInterface|Viewport|AddtoViewport _returnvalue_2 0)
  (Actor|DestroyActor))

(event EventBeginPlay
  (bind _returnvalue (SaveGame|LoadGamefromSlot "Save"))
  (bind _assg_save_data (Utilities|Casting|CastToSG_SaveData _returnvalue))
  (if (> (Variables|/Game/Blueprints/SaveGame/SG_SaveData.SG_SaveData_C|GetHealthHealAMT _assg_save_data) 2)
    (Actor|DestroyActor)))

(fn ConstructionScript)