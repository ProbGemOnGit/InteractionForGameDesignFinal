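; BP_SavePoint is a crystal checkpoint that saves the player's respawn location on overlap.
; It writes its arrow's location to the "Save" slot, messages the player, and refreshes their heal item if not already active.
; Activation cancels every save point in the world, then swaps its own crystal materials.
; While JustSpawned holds, cleared two seconds after BeginPlay, overlap also starts the area's music through the game mode.
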(event OnComponentBeginOverlap(Box)
  (params (OverlappedComponent :type Primitive%20Component%20Object%20Reference) (OtherActor :type Actor%20Object%20Reference) (OtherComp :type Primitive%20Component%20Object%20Reference) (OtherBodyIndex :type Integer) (bFromSweep :type Boolean) (SweepResult :type Hit%20Result%20Structure%20%28by%20ref%29))
  ;[0.15 0.15 0.15 0.5] If overlaped with player sets new spawn point in save data in save data
  (if (Actor|ActorHasTag OtherActor "Player")
    (bind _returnvalue (SaveGame|LoadGamefromSlot "Save"))
    (bind _assg_save_data (Utilities|Casting|CastToSG_SaveData _returnvalue))
    (Variables|/Game/Blueprints/SaveGame/SG_SaveData.SG_SaveData_C|SetCheckPointLocation _assg_save_data (Transformation|GetWorldLocation (Variables|Default|GetArrow)))
    (SaveGame|SaveGametoSlot _assg_save_data "Save")
    (Class|BPIPlayer|SetNewSpawnLocation(Message) OtherActor (Transformation|GetWorldLocation (Variables|Default|GetArrow)))
    (if (Variables|Default|GetIsSavePoint)
      _
      (else
        (Class|BPIPlayer|RefreshHealItem(Message) OtherActor)))
    (CallFunction|SetSavePoint)
    (if (Variables|Default|GetJustSpawned)
      (switch Utilities|FlowControl|Switch|SwitchonE_Music (Variables|Default|GetMusic)
        (:NewEnumerator0
          (bind _asbp_research_project_game_mode (Utilities|Casting|CastToBP_ResearchProjectGameMode (Game|GetGameMode)))
          (Default|ActivateMusic _asbp_research_project_game_mode "/Game/SoundEffects/Music/Cave_of_Apprehension_Favorite_1.Cave_of_Apprehension_Favorite_1"))
        (:NewEnumerator1
          (bind _asbp_research_project_game_mode_2 (Utilities|Casting|CastToBP_ResearchProjectGameMode (Game|GetGameMode)))
          (Default|ActivateMusic _asbp_research_project_game_mode_2 "/Game/SoundEffects/Music/Crystal_Cavern_Reverie_Favorite_1.Crystal_Cavern_Reverie_Favorite_1"))
        (:NewEnumerator2
          (bind _asbp_research_project_game_mode_3 (Utilities|Casting|CastToBP_ResearchProjectGameMode (Game|GetGameMode)))
          (Default|ActivateMusic _asbp_research_project_game_mode_3 "/Game/SoundEffects/Music/DungeonMusic.DungeonMusic"))))))

(event Custom|SetSavePoint
  ;[0.15 0.15 0.15 0.5] Sets save point and removes other save points in the world
  (bind _outactors (Actor|GetAllActorsOfClass "BP_SavePoint_C"))
  (for _array_element _outactors
    (CallFunction|CancelSavePoint _array_element))
  (Rendering|Material|SetMaterial (Variables|Default|GetCrystalModel) 0 "/Game/effects/crystal/Crystal_MAT_2.Crystal_MAT_2")
  (Variables|Default|SetIsSavePoint true))

(event Custom|CancelSavePoint
  ;[0.15 0.15 0.15 0.5] cancels THIS savepoint when called
  (Rendering|Material|SetMaterial (Variables|Default|GetCrystalModel) 0 "/Game/effects/crystal/Crystal_MAT_1.Crystal_MAT_1")
  (Variables|Default|SetIsSavePoint false))

(event EventBeginPlay
  (Utilities|FlowControl|Delay 2.0)
  (Variables|Default|SetJustSpawned false))

(fn ConstructionScript)