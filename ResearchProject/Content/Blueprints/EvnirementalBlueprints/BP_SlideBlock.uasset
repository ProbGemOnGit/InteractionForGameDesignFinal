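; BP_SlideBlock is an environmental block actor whose presence in the level depends on saved game state.
; On BeginPlay it loads SG_SaveData from the "Save" slot and checks the SlideBlockActive flag.
; If active, it teleports and rescales its Cube and Box collider from stored location and size variables; otherwise it destroys itself.
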(event EventBeginPlay
  (bind _cube (Variables|Default|GetCube))
  (bind _box (Variables|Default|GetBox))
  (bind _returnvalue (SaveGame|LoadGamefromSlot "Save"))
  (bind _assg_save_data (Utilities|Casting|CastToSG_SaveData _returnvalue))
  (if (Variables|/Game/Blueprints/SaveGame/SG_SaveData.SG_SaveData_C|GetSlideBlockActive _assg_save_data)
    (Transformation|SetWorldLocation _cube (Variables|Default|GetLocatyion) false true)
    (Transformation|SetWorldScale3D _cube (Variables|Default|GetBlockSize))
    (Transformation|SetWorldLocation _box (Variables|Default|GetColliderLocation) false true)
    (Transformation|SetWorldScale3D _box (Variables|Default|GetColliderSize))
    (else
      (Actor|DestroyActor))))

(fn ConstructionScript)