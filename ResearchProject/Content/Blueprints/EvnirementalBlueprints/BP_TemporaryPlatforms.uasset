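; BP_TemporaryPlatforms is a hittable trigger that spawns a set of temporary platforms when its HitActor event fires.
; HitActor spawns a BP_Platform at each transform in the Platforms array, records it in SpawnPlatforms and starts a timer of TimeForPlatforms.
; When the timer fires, it destroys the valid spawned platforms and restores CanHitObject, which blocks repeat hits while they exist.
; SpawnPlatforms is never cleared, so the IsValid check skips entries from earlier cycles.
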(event Custom|CustomEvent
  (for _array_element (Variables|Default|GetSpawnPlatforms)
    (Utilities|IsValid _array_element
      (:Is%20Valid
        (Actor|DestroyActor _array_element))))
  (Variables|Default|SetCanHitObject true))

(event EventHitActor
  (params (Damage :type Integer))
  (Development|PrintString "Hello")
  (if (Variables|Default|GetCanHitObject)
    (Variables|Default|SetCanHitObject false)
    (for _array_element (Variables|Default|GetPlatforms)
      (bind _returnvalue (Game|SpawnActorfromClass "/Game/Blueprints/EvnirementalBlueprints/BP_Platform.BP_Platform_C" _array_element "Undefined" "MultiplyWithRoot" 0 0))
      (Utilities|Array|Add (Variables|Default|GetSpawnPlatforms) _returnvalue))
    (Utilities|Time|SetTimerbyEvent (delegate Custom|CustomEvent) (Variables|Default|GetTimeForPlatforms))))

(fn ConstructionScript)