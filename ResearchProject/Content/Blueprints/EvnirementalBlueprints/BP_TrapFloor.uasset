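; BP_TrapFloor is a one-time cave floor trap that collapses under the player and removes itself on load once the save marks it gone.
; One overlap box restricts the player to walking; the other halts movement, disables input, updates the save and spawns a BP_SlideBlock at a hardcoded location.
; After short delays it destroys its floor meshes, restores input and normal movement, then destroys itself.
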(event OnComponentBeginOverlap(Box)
  (params (OverlappedComponent :type Primitive%20Component%20Object%20Reference) (OtherActor :type Actor%20Object%20Reference) (OtherComp :type Primitive%20Component%20Object%20Reference) (OtherBodyIndex :type Integer) (bFromSweep :type Boolean) (SweepResult :type Hit%20Result%20Structure%20%28by%20ref%29))
  (bind _returnvalue (Game|GetPlayerController 0))
  (bind _asbp_research_project_character (Utilities|Casting|CastToBP_ResearchProjectCharacter OtherActor))
  (Utilities|Casting|CastToPlatformerMovementComponent (Variables|/Script/Engine.Character|GetCharacterMovement _asbp_research_project_character))
  (Components|Movement|StopMovementImmediately (Variables|/Script/Engine.Character|GetCharacterMovement _asbp_research_project_character))
  (Input|DisableInput (Game|GetPlayerController 0))
  (bind _returnvalue_2 (SaveGame|LoadGamefromSlot "Save"))
  (bind _assg_save_data (Utilities|Casting|CastToSG_SaveData _returnvalue_2))
  (Variables|/Game/Blueprints/SaveGame/SG_SaveData.SG_SaveData_C|SetIsCaveDropFloorPresent? _assg_save_data false)
  (Variables|/Game/Blueprints/SaveGame/SG_SaveData.SG_SaveData_C|SetSlideBlockActive _assg_save_data true)
  (SaveGame|SaveGametoSlot _assg_save_data "Save")
  (Game|SpawnActorfromClass "/Game/Blueprints/EvnirementalBlueprints/BP_SlideBlock.BP_SlideBlock_C" (Math|Transform|MakeTransform "9930.000000,380.000000,1980.000000" "0, 0, 0" "1.000000,1.000000,1.000000") "Undefined" "MultiplyWithRoot" 0 "10.800000,14.799970,2.000000" "9930.000000,380.000000,1980.000000" "10.800600,14.799970,2.000000" "1.471100,20.000000,8.999000" 0)
  (Input|DisableInput _asbp_research_project_character _returnvalue)
  (Utilities|FlowControl|Delay 1.0)
  (Components|DestroyComponent (Variables|Default|GetStaticMesh))
  (Utilities|FlowControl|Delay 2.0)
  (Input|EnableInput _asbp_research_project_character _returnvalue)
  (Default|WalkOnly _asbp_research_project_character false)
  (Actor|DestroyActor))

(event OnComponentBeginOverlap(Box1)
  (params (OverlappedComponent :type Primitive%20Component%20Object%20Reference) (OtherActor :type Actor%20Object%20Reference) (OtherComp :type Primitive%20Component%20Object%20Reference) (OtherBodyIndex :type Integer) (bFromSweep :type Boolean) (SweepResult :type Hit%20Result%20Structure%20%28by%20ref%29))
  (bind _asbp_research_project_character (Utilities|Casting|CastToBP_ResearchProjectCharacter OtherActor))
  (Default|WalkOnly _asbp_research_project_character true))

(event EventBeginPlay
  (bind _returnvalue (SaveGame|LoadGamefromSlot "Save"))
  (bind _assg_save_data (Utilities|Casting|CastToSG_SaveData _returnvalue))
  (if (not (Variables|/Game/Blueprints/SaveGame/SG_SaveData.SG_SaveData_C|GetIsCaveDropFloorPresent? _assg_save_data))
    (Actor|DestroyActor)))

(fn ConstructionScript)