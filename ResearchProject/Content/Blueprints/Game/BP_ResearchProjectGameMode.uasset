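; Game mode that persists the player's checkpoint and save point between sessions and controls a single 2D music track.
; Checkpoint location and save point name are written to text files in the project Saved directory.
; On BeginPlay it reads them back, teleports the player capsule to the checkpoint and reactivates the BP_SavePoint matched by object name.
; Music events fade the sound in and out, with a DoOnce preventing duplicate starts.
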(event Custom|ActivateMusic
  (params (Sound :type Sound%20Base%20Object%20Reference))
  (Utilities|FlowControl|DoOnce false
    (:Completed
      (bind _returnvalue (Audio|SpawnSound2D Sound 1.0 1.0 0.0 0))
      (Variables|Default|SetMusic _returnvalue)
      (Variables|Default|SetMusicIsPlaying true)
      (Audio|Components|Audio|FadeIn (Variables|Default|GetMusic) 1.0 1.0 0.0 "Linear" :!class /Script/Engine.AudioComponent))))

(event Custom|DeactivateMusic
  (params (Sound :type Sound%20Base%20Object%20Reference))
  (if (Variables|Default|GetMusicIsPlaying)
    (Variables|Default|SetMusicIsPlaying false)
    (Audio|Components|Audio|FadeOut (Variables|Default|GetMusic) 1.0 0.0 "Linear" :!class /Script/Engine.AudioComponent)
    (Utilities|FlowControl|DoOnce false) ; enters at Reset
    (else
      (Utilities|FlowControl|DoOnce false) ; enters at Reset
    )))

(event Custom|SaveCheckPointLocation
  (params (Saved%20Location :type String))
  (Class|CPPSaveGame|WritetoFile (Class|KismetSystemLibrary|GetProjectSavedDirectory) "PlayerLocation.txt" Saved%20Location))

(event Custom|GetCheckPpointLocation
  (bind (_boutsuccess _boutmessage _returnvalue) (Class|CPPSaveGame|ReadfromFile (Class|KismetSystemLibrary|GetProjectSavedDirectory) "PlayerLocation.txt"))
  (if _boutsuccess
    (if (.OutIsValid (Math|Conversions|ToVector(Float) _returnvalue))
      (Variables|Default|SetCheckPointLocation (.OutConvertedVector (Math|Conversions|ToVector(Float) _returnvalue))))))

(event Custom|SaveSavePoint
  (params (SavePointName :type String))
  (Variables|Default|SetSavePoint SavePointName)
  (Class|CPPSaveGame|WritetoFile (Class|KismetSystemLibrary|GetProjectSavedDirectory) "SavePoint.txt" SavePointName))

(event Custom|LoadSavePoint
  (bind (_boutsuccess _boutmessage _returnvalue) (Class|CPPSaveGame|ReadfromFile (Class|KismetSystemLibrary|GetProjectSavedDirectory) "SavePoint.txt"))
  (if _boutsuccess
    (bind _outactors (Actor|GetAllActorsOfClass "/Game/Blueprints/EvnirementalBlueprints/BP_SavePoint.BP_SavePoint_C"))
    (bind _array_element (Utilities|Array|ForEachLoopwithBreak _outactors)
      (:LoopBody
        (if (Utilities|Enum|Equal(Enum) (Utilities|GetObjectName _array_element) _boutmessage)
          (Default|SetSavePoint _array_element)))
      (:Completed
        (Variables|Default|SetSavePoint _returnvalue)))))

(event EventBeginPlay
  (bind _returnvalue (Game|GetPlayerCharacter 0))
  (CallFunction|GetCheckPpointLocation)
  (Utilities|IsValid _returnvalue
    (:Is%20Valid
      (Transformation|SetWorldLocation (Variables|/Script/Engine.Character|GetCapsuleComponent _returnvalue) (Variables|Default|GetCheckPointLocation) false true)
      (CallFunction|LoadSavePoint))))

(fn ConstructionScript)