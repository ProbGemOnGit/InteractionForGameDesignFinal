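; BP_BossAi is the boss actor for the boss fight, starting its attack behavior when woken.
; On BeginPlay it attaches the sword and staff to hand sockets and spawns a BP_BossAreaEffect, stored as its ground slam spikes.
; WakeUp clears the dormant flag, sets capsule collision to overlap pawns and a custom channel, then after a short delay raises the attacking and jump attack flags.
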(event Custom|WakeUp
  (bind _capsulecomponent (Variables|Collision|GetCapsuleComponent))
  (Variables|Default|SetIsDormant false)
  (Collision|SetCollisionResponsetoChannel _capsulecomponent "ECC_Pawn" "ECR_Overlap")
  (Collision|SetCollisionResponsetoChannel _capsulecomponent "ECC_GameTraceChannel3" "ECR_Overlap")
  (Utilities|FlowControl|Delay 3.0)
  (Variables|Default|SetIsAttacking true)
  (Variables|Default|SetJumpAttack true))

(event EventBeginPlay
  (Transformation|AttachComponentToComponent (Variables|Default|GetSword) (Variables|Character|GetMesh) "hand_rSocket" "SnapToTarget" "SnapToTarget" "KeepRelative" true)
  (Transformation|AttachComponentToComponent (Variables|Default|GetStaff) (Variables|Character|GetMesh) "hand_lSocket" "SnapToTarget" "SnapToTarget" "KeepRelative" true)
  (bind _returnvalue (Game|SpawnActorfromClass "/Game/BossFight/Boss/BP_BossAreaEffect.BP_BossAreaEffect_C" (Math|Transform|MakeTransform "0, 0, 0" "0, 0, 0" "1.000000,1.000000,1.000000") "Undefined" "MultiplyWithRoot" 0 0))
  (Variables|Default|SetGroundSlamSpikes _returnvalue))

(fn ConstructionScript)