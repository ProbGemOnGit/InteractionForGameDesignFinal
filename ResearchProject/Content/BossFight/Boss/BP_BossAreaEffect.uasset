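; Boss fight area attack that stays hidden until TriggerSpikes reveals it and raises two spike meshes outward from below on a timeline.
; When the rise finishes, HurtBox checks actors overlapping two capsules and sends a one-damage hit message to the first one tagged Player.
; After a short delay, a second timeline retracts the spikes and hides the effect again.
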(event Custom|HurtBox
  (bind _output_get (Variables|Default|SetOverlapping%20Actors (Collision|GetOverlappingActors (Variables|Default|GetCapsule1) 0 :!class /Script/Engine.PrimitiveComponent)))
  (Utilities|Array|AppendArray _output_get (Collision|GetOverlappingActors (Variables|Default|GetCapsule) 0 :!class /Script/Engine.PrimitiveComponent))
  (bind _array_element (Utilities|Array|ForEachLoopwithBreak (Variables|Default|GetOverlapping%20Actors) :!label _label)
    (:LoopBody
      (if (Actor|ActorHasTag _array_element "Player")
        (Class|BPIPlayer|HitPlayer(Message) _array_element 1 (Transformation|GetWorldLocation (Variables|Default|GetDefaultSceneRoot)))
        (goto _label Break)))
    (:Completed
      (Utilities|FlowControl|Delay 1.0)
      (bind _newtrack_0 (Timeline|Timeline_0 PlayFromStart)
        (:Update
          (Transformation|SetRelativeLocation (Variables|Default|GetStaticMesh) (Math|Vector|Lerp(Vector) "-125.000000,0.000000,60.000000" "7.000000,0.000000,-170.000000" _newtrack_0) false false)
          (Transformation|SetRelativeLocation (Variables|Default|GetStaticMesh2) (Math|Vector|Lerp(Vector) "125.000000,0.000000,60.000000" "-7.000000,0.000000,-170.000000" _newtrack_0) false false))
        (:Finished
          (Rendering|SetVisibility (Variables|Default|GetDefaultSceneRoot) false true))))))

(event Custom|TriggerSpikes
  (Rendering|SetVisibility (Variables|Default|GetDefaultSceneRoot) true true)
  (bind _newtrack_0 (Timeline|Timeline PlayFromStart)
    (:Update
      (Transformation|SetRelativeLocation (Variables|Default|GetStaticMesh) (Math|Vector|Lerp(Vector) "7.000000,0.000000,-170.000000" "-125.000000,0.000000,60.000000" _newtrack_0) false false)
      (Transformation|SetRelativeLocation (Variables|Default|GetStaticMesh2) (Math|Vector|Lerp(Vector) "-7.000000,0.000000,-170.000000" "125.000000,0.000000,60.000000" _newtrack_0) false false))
    (:Finished
      (CallFunction|HurtBox))))

(event EventBeginPlay
  (Rendering|SetVisibility (Variables|Default|GetDefaultSceneRoot) false true))

(fn ConstructionScript)