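; Boss ground-crystal attack actor that sends out a sphere, raises three spikes from the ground, then destroys itself.
; On BeginPlay, chained timelines lerp the sphere from its start location to an arrow marker, then raise the spikes one after another, hiding the sphere after the first.
; After a short delay, one timeline sinks all spikes together.
; Two capsule overlaps send a hit-player interface message with damage and an arrow's location.
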(event OnComponentBeginOverlap(Capsule1)
  (params (OverlappedComponent :type Primitive%20Component%20Object%20Reference) (OtherActor :type Actor%20Object%20Reference) (OtherComp :type Primitive%20Component%20Object%20Reference) (OtherBodyIndex :type Integer) (bFromSweep :type Boolean) (SweepResult :type Hit%20Result%20Structure%20%28by%20ref%29))
  ;[0.15 0.15 0.15 0.5] If player overlaps with crystals triggers hit player interface
  (Class|BPIPlayer|HitPlayer(Message) OtherActor 1 (Transformation|GetWorldLocation (Variables|Default|GetArrow))))

(event OnComponentBeginOverlap(Capsule)
  (params (OverlappedComponent :type Primitive%20Component%20Object%20Reference) (OtherActor :type Actor%20Object%20Reference) (OtherComp :type Primitive%20Component%20Object%20Reference) (OtherBodyIndex :type Integer) (bFromSweep :type Boolean) (SweepResult :type Hit%20Result%20Structure%20%28by%20ref%29))
  ;[0.15 0.15 0.15 0.5] If player overlaps with crystals triggers hit player interface
  (Class|BPIPlayer|HitPlayer(Message) OtherActor 1 (Transformation|GetWorldLocation (Variables|Default|GetArrow))))

(event Custom|TriggerSpikes
  ;[0.15 0.15 0.15 0.5] Moves the 3 spikes out of the ground back to back to back
  (bind _newtrack_0 (Timeline|Timeline_3 PlayFromStart)
    (:Update
      (Transformation|SetRelativeLocation (Variables|Default|GetStaticMesh4) (Math|Vector|Lerp(Vector) "95.000000,0.000000,-200.000000" "116.000000,0.000000,-85.000000" _newtrack_0) false false))
    (:Finished
      (Rendering|SetVisibility (Variables|Default|GetSphere) false true)
      (bind _newtrack_0_2 (Timeline|Timeline PlayFromStart)
        (:Update
          (Transformation|SetRelativeLocation (Variables|Default|GetStaticMesh2) (Math|Vector|Lerp(Vector) "180.000000,0.000000,-200.000000" "360.000000,0.000000,60.000000" _newtrack_0_2) false false))
        (:Finished
          (bind _newtrack_0_3 (Timeline|Timeline_1 PlayFromStart)
            (:Update
              (Transformation|SetRelativeLocation (Variables|Default|GetStaticMesh) (Math|Vector|Lerp(Vector) "130.000000,0.000000,-200.000000" "450.000000,0.000000,-15.000000" _newtrack_0_3) false false))
            (:Finished
              (Utilities|FlowControl|Delay 0.2)
              (CallFunction|ShrinkandDestroy))))))))

(event Custom|ShrinkAndDestroy
  ;[0.15 0.15 0.15 0.5] shricks the spikes into the ground and then destroys object
  (bind _newtrack_0 (Timeline|Timeline_0 PlayFromStart)
    (:Update
      (Transformation|SetRelativeLocation (Variables|Default|GetStaticMesh) (Math|Vector|Lerp(Vector) "450.000000,0.000000,-15.000000" "130.000000,0.000000,-200.000000" _newtrack_0) false false)
      (Transformation|SetRelativeLocation (Variables|Default|GetStaticMesh2) (Math|Vector|Lerp(Vector) "360.000000,0.000000,60.000000" "180.000000,0.000000,-200.000000" _newtrack_0) false false)
      (Transformation|SetRelativeLocation (Variables|Default|GetStaticMesh4) (Math|Vector|Lerp(Vector) "116.000000,0.000000,-85.000000" "95.000000,0.000000,-200.000000" _newtrack_0) false false))
    (:Finished
      (Rendering|SetVisibility (Variables|Default|GetDefaultSceneRoot) false true)
      (Actor|DestroyActor))))

(event EventBeginPlay
  ;[0.15 0.15 0.15 0.5] On begin play moves the crystal shpere to a position in front of the boss
  (bind _newtrack_0 (Timeline|Timeline_2 PlayFromStart)
    (:Update
      (Transformation|SetWorldLocation (Variables|Default|GetSphere) (Math|Vector|Lerp(Vector) (Variables|Default|GetStartSphereLocation) (Transformation|GetWorldLocation (Variables|Default|GetArrow1)) _newtrack_0) false false))
    (:Finished
      (CallFunction|TriggerSpikes))))

(fn ConstructionScript)