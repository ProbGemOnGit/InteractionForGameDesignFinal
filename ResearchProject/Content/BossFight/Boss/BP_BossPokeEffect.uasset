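; BP_BossPokeEffect is a short-lived crystal poke attack effect for the boss fight that damages what it hits.
; On BeginPlay, three chained timelines grow the mesh, thrust it along local X after a brief delay, then shrink it before the actor destroys itself.
; A capsule overlap sends the HitPlayer interface message to the other actor with one damage and the arrow component's world location, without filtering for the player.
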(event OnComponentBeginOverlap(Capsule1)
  (params (OverlappedComponent :type Primitive%20Component%20Object%20Reference) (OtherActor :type Actor%20Object%20Reference) (OtherComp :type Primitive%20Component%20Object%20Reference) (OtherBodyIndex :type Integer) (bFromSweep :type Boolean) (SweepResult :type Hit%20Result%20Structure%20%28by%20ref%29))
  ;[0.15 0.15 0.15 0.5] If player overlaps with crystal triggers hit player interface
  (Class|BPIPlayer|HitPlayer(Message) OtherActor 1 (Transformation|GetWorldLocation (Variables|Default|GetArrow))))

(event EventBeginPlay
  ;[0.15 0.15 0.15 0.5] On begin play triggers crystal poking animation
  (bind _newtrack_0 (Timeline|Timeline PlayFromStart)
    (:Update
      (Transformation|SetRelativeScale3D (Variables|Default|GetStaticMesh) (Math|Vector|Lerp(Vector) "0.100000,0.100000,0.100000" "35.000000,35.000000,35.000000" _newtrack_0)))
    (:Finished
      (Utilities|FlowControl|Delay 0.2)
      (bind _newtrack_0_2 (Timeline|Timeline_0 PlayFromStart)
        (:Update
          (Transformation|SetRelativeLocation (Variables|Default|GetStaticMesh) (Math|Vector|Lerp(Vector) "-170.000000,0.000000,0.000000" "220.000000,0.000000,-0.000000" _newtrack_0_2) false false))
        (:Finished
          (bind _newtrack_0_3 (Timeline|Timeline_1 PlayFromStart)
            (:Update
              (Transformation|SetRelativeScale3D (Variables|Default|GetStaticMesh) (Math|Vector|Lerp(Vector) "35.000000,35.000000,35.000000" "0.100000,0.100000,0.100000" _newtrack_0_3)))
            (:Finished
              (Actor|DestroyActor))))))))

(fn ConstructionScript)