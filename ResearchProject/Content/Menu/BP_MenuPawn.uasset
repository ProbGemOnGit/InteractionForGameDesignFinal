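; BP_MenuPawn is the main menu pawn that adds the input mapping and shows the MainMenuWBP1 widget on begin play.
; Vertical IA_Move input steps a selection clamped between three entries and pushes it to the widget through UpdateMenu.
; A latch flag allows one step per stick push until the input falls back below the threshold.
; IA_Jump confirms the current choice by calling the widget's SelectMenu.
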(event Input|EnhancedActionEvents|EnhancedInputActionIA_Move
  (params (ActionValue :type Vector%202D%20Structure) (ElapsedSeconds :type Float%20%28double-precision%29) (TriggeredSeconds :type Float%20%28double-precision%29) (InputAction :type Input%20Action%20Object%20Reference :default "/Game/Input/Actions/IA_Move.IA_Move"))
  (if (> (Math|Float|Absolute(Float) (.y ActionValue)) 0.8)
    (if (Variables|Default|GetCanChangedChoice)
      (if (< (.y ActionValue) 0.0)
        (Math|Integer|IncrementInt (Variables|Default|GetSelection)
          (:%20%20
            (if (> (Variables|Default|GetSelection) 3)
              (Variables|Default|SetSelection 3))))
        (else
          (Math|Integer|DecrementInt (Variables|Default|GetSelection)
            (:%20%20
              (if (< (Variables|Default|GetSelection) 1)
                (Variables|Default|SetSelection 1))))))
      (Default|UpdateMenu (Variables|Default|GetMenu) (Variables|Default|GetSelection))
      (Variables|Default|SetCanChangedChoice false))
    (else
      (Variables|Default|SetCanChangedChoice true))))

(event Input|EnhancedActionEvents|EnhancedInputActionIA_Jump
  (params (ActionValue :type Boolean) (ElapsedSeconds :type Float%20%28double-precision%29) (TriggeredSeconds :type Float%20%28double-precision%29) (InputAction :type Input%20Action%20Object%20Reference :default "/Game/Input/Actions/IA_Jump.IA_Jump"))
  (:Started
    (Default|SelectMenu (Variables|Default|GetMenu))))

(event EventBeginPlay
  (Input|AddMappingContext (PlayerController|LocalPlayerSubsystems|GetEnhancedInputLocalPlayerSubsystem (Game|GetPlayerController 0)) "/Game/Input/IMC_Default.IMC_Default" 0 "(bIgnoreAllPressedKeysUntilRelease=True,bForceImmediately=False,bNotifyUserSettings=False)")
  (bind _returnvalue (UserInterface|CreateWidget "/Game/UI/MenuAssets/MainMenuWBP1.MainMenuWBP1_C"))
  (UserInterface|Viewport|AddtoViewport _returnvalue 0)
  (Variables|Default|SetMenu _returnvalue))

(fn ConstructionScript)